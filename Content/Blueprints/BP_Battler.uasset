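; Team-coloured battler that visually plays out turn actions: moving to a tile or shooting at a target location.
; InitTeam creates a dynamic material coloured red or blue, which turns grey on death and animates a damage effect when hit.
; StartAction scales timeline play rates by the inverse of DeltaTime to lerp either the actor or a spawned BP_Bullet to the target, destroying the bullet on arrival.
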(event Custom|OnDiedEvent
  (Rendering|Material|SetVectorParameterValue (Variables|Default|GetDynMat) "Colour" "(R=0.218750,G=0.218750,B=0.218750,A=1.000000)" :!class /Script/Engine.MaterialInstanceDynamic))

(event Custom|OnDamagedEvent
  (bind _damagedalpha (Timeline|DamagedTimeline PlayFromStart)
    (:Update
      (Rendering|Material|SetScalarParameterValue (Variables|Default|GetDynMat) "DamagedAlpha" _damagedalpha :!class /Script/Engine.MaterialInstanceDynamic))))

(event EventBeginPlay
  (|CallParentFunction)
  (EventDispatchers|BindEventtoOnDied (EventDispatchers|CreateEvent :!event Custom|OnDiedEvent))
  (EventDispatchers|BindEventtoOnDamaged (EventDispatchers|CreateEvent :!event Custom|OnDamagedEvent)))

(event EventInitTeam
  (params (Team :type ETeam%20Enum :default "Red"))
  (|CallParentFunction Team)
  (bind _returnvalue (Rendering|Material|CreateDynamicMaterialInstance "/Game/Materials/M_Battler.M_Battler" "None" "None" :!class /Script/Engine.KismetMaterialLibrary))
  (bind _output_get (Variables|Default|SetDynMat _returnvalue))
  (Rendering|Material|SetVectorParameterValue _returnvalue "Colour" (Utilities|Select :Index (Variables|Default|GetTeamName) :Red "(R=1.000000,G=0.000000,B=0.000000,A=1.000000)" :Blue "(R=0.000000,G=0.000000,B=0.990000,A=1.000000)") :!class /Script/Engine.MaterialInstanceDynamic)
  (Rendering|Material|SetMaterial (Variables|Default|GetStaticMeshComp) 0 (Variables|Default|GetDynMat)))

(event EventStartAction
  (params (TargetLocation :type Vector :default "0, 0, 0") (DeltaTime :type Float%20%28single-precision%29))
  (Variables|Default|SetTarget%20Location TargetLocation)
  (Variables|Default|SetCurrentLocation (Transformation|GetActorLocation))
  (switch Utilities|FlowControl|Switch|SwitchonETurnMode (Variables|Default|GetTurnMode)
    (:MoveToNextTile
      (Components|Timeline|SetPlayRate (Variables|Default|GetTimeline) (/ 1.0 DeltaTime))
      (bind _alpha (Timeline|Timeline PlayFromStart)
        (:Update
          (Transformation|SetActorLocation (Math|Vector|Lerp(Vector) (Variables|Default|GetCurrentLocation) (Variables|Default|GetTarget%20Location) _alpha) false false))))
    (:Attack
      (bind _returnvalue (Game|SpawnActorfromClass "/Game/Blueprints/BP_Bullet.BP_Bullet_C" (Transformation|GetActorTransform) "Undefined" 0 0))
      (Components|Timeline|SetPlayRate (Variables|Default|GetTimeline_0) (/ 1.0 DeltaTime))
      (bind _alpha_2 (Timeline|Timeline_0 PlayFromStart)
        (:Update
          (Transformation|SetActorLocation _returnvalue (Math|Vector|Lerp(Vector) (Variables|Default|GetCurrentLocation) (Variables|Default|GetTarget%20Location) _alpha_2) false false))
        (:Finished
          (Actor|DestroyActor _returnvalue))))))

(fn ConstructionScript)